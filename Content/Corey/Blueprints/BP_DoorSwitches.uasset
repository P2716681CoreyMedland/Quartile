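; BP_DoorSwitches is a door that opens once enough pressure switches are active at the same time.
; Switch activate and deactivate events adjust a running count and compare it to the required number.
; The DoorMovement timeline drives the door's relative Z, playing when the requirement is met and reversing otherwise.
; A separate DoorOpen event moves the door through its own timeline, independent of the count.
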(event `DoorOpen`
  (bind (_direction _doorpos) (`Timeline|Timeline`)
    (:`Update`
      (`SceneComponent.K2_SetRelativeLocation` (`self.Door`) (`KismetMathLibrary.MakeVector` 0.0 0.0 _doorpos) false false))))

(event `SwitchActivated`
  (`/Engine/EditorBlueprintResources/StandardMacros.IncrementInt` (`self.PressureSwitchesActive`)
    (:`  `
      (if (>= (`self.PressureSwitchesActive`) (`self.PressureSwitchesNeeded`))
        (bind (_direction _doorpos) (`Timeline|DoorMovement` :!label _label)
          (:`Update`
            (`SceneComponent.K2_SetRelativeLocation` (`self.Door`) (`KismetMathLibrary.MakeVector` 0.0 0.0 _doorpos) false false)))
        (else
          (goto _label :!via `Reverse`))))))

(event `SwitchDeactivated`
  (`/Engine/EditorBlueprintResources/StandardMacros.DecrementInt` (`self.PressureSwitchesActive`)
    (:`  `
      (if (>= (`self.PressureSwitchesActive`) (`self.PressureSwitchesNeeded`))
        (goto _label)
        (else
          (goto _label :!via `Reverse`))))))

(fn `UserConstructionScript`)