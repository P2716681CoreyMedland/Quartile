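; BP_NPC is a dialogue NPC that starts a conversation with C_PlayerCharacter on actor overlap and ends it when the overlap ends.
; Decision stores the player's chosen option, and Consequences branches on it, always updating the reply from NPCConsequences through the player's WBP_Talk widget.
; The second option also opens the linked Door, and both second and third options end the talk after a short delay.
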(event `self.ReceiveActorBeginOverlap`
  (params (OtherActor :type "Actor Object Reference"))
  (bind _asc_player_character (cast `/Game/Player/C_PlayerCharacter` (`GameplayStatics.GetPlayerCharacter` 0)))
  (`/Game/Player/C_PlayerCharacter.Talk` _asc_player_character self))

(event `self.ReceiveActorEndOverlap`
  (params (OtherActor :type "Actor Object Reference"))
  (bind _asc_player_character (cast `/Game/Player/C_PlayerCharacter` (`GameplayStatics.GetPlayerCharacter` 0)))
  (`/Game/Player/C_PlayerCharacter.EndTalk` _asc_player_character))

(event `Decision`
  (params (PlayerDecision :type "/Game/Corey/Blueprints/NPC/Blueprints/E_PlayerOptions Enum" :default "NewEnumerator0"))
  (set `self.E_PlayerOptions` PlayerDecision)
  (`self.Consequences`))

(event `Consequences`
  (switch `/Game/Corey/Blueprints/NPC/Blueprints/E_PlayerOptions` (`self.E_PlayerOptions`)
    (:`NewEnumerator0`
      (`self.Update NPC Reply`))
    (:`NewEnumerator1`
      (`self.Update NPC Reply`)
      (`/Game/Corey/Blueprints/BP_DoorSwitches.DoorOpen` (`self.Door`))
      (`KismetSystemLibrary.Delay` 1.5)
      (bind _asc_player_character (cast `/Game/Player/C_PlayerCharacter` (`GameplayStatics.GetPlayerCharacter` 0)))
      (`/Game/Player/C_PlayerCharacter.EndTalk` _asc_player_character))
    (:`NewEnumerator2`
      (`self.Update NPC Reply`)
      (`KismetSystemLibrary.Delay` 1.5)
      (bind _asc_player_character_2 (cast `/Game/Player/C_PlayerCharacter` (`GameplayStatics.GetPlayerCharacter` 0)))
      (`/Game/Player/C_PlayerCharacter.EndTalk` _asc_player_character_2))))

(event `Update NPC Reply`
  (set `self.NPC_Reply` (`|GetArrayItem` (`self.NPC_Consequences`) (`KismetMathLibrary.Conv_ByteToInt` (`self.E_PlayerOptions`))))
  (bind _asc_player_character (cast `/Game/Player/C_PlayerCharacter` (`GameplayStatics.GetPlayerCharacter` 0)))
  (bind _aswbp_talk (cast `/Game/Corey/Blueprints/NPC/Blueprints/WBP_Talk` (`/Game/Player/C_PlayerCharacter.UI_Talk` _asc_player_character)))
  (`/Game/Corey/Blueprints/NPC/Blueprints/WBP_Talk.Update Reply` _aswbp_talk self))

(fn `UserConstructionScript`)