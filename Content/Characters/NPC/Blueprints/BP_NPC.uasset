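; BP_NPC is an NPC actor that starts dialogue with the player character and replies to their chosen option.
; Any actor overlap calls Talk on the player's BP_ThirdPersonCharacter, passing itself.
; Decision stores the chosen EPlayerOptions value, and all three option branches in Consequences run the same reply update.
; That update picks NPCReply from NPCConsequences by enum index and refreshes the player's WBP_Talk widget.
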(event `self.ReceiveActorBeginOverlap`
  (params (OtherActor :type "Actor Object Reference"))
  (bind _asbp_third_person_character (cast `/Game/ThirdPerson/Blueprints/BP_ThirdPersonCharacter` (`GameplayStatics.GetPlayerCharacter` 0)))
  (`/Game/ThirdPerson/Blueprints/BP_ThirdPersonCharacter.Talk` _asbp_third_person_character self))

(event `Decision`
  (params (PlayerDecision :type "/Game/Characters/NPC/Blueprints/E_PlayerOptions Enum" :default "NewEnumerator0"))
  (set `self.E_PlayerOptions` PlayerDecision)
  (`self.Consequences`))

(event `Consequences`
  (switch `/Game/Characters/NPC/Blueprints/E_PlayerOptions` (`self.E_PlayerOptions`)
    (:`NewEnumerator0`
      (`self.Update NPC Reply`))
    (:`NewEnumerator1`
      (`self.Update NPC Reply`))
    (:`NewEnumerator2`
      (`self.Update NPC Reply`))))

(event `Update NPC Reply`
  (set `self.NPC_Reply` (`|GetArrayItem` (`self.NPC_Consequences`) (`KismetMathLibrary.Conv_ByteToInt` (`self.E_PlayerOptions`))))
  (bind _asbp_third_person_character (cast `/Game/ThirdPerson/Blueprints/BP_ThirdPersonCharacter` (`GameplayStatics.GetPlayerCharacter` 0)))
  (bind _aswbp_talk (cast `/Game/Characters/NPC/Blueprints/WBP_Talk` (`/Game/ThirdPerson/Blueprints/BP_ThirdPersonCharacter.UI_Talk` _asbp_third_person_character)))
  (`/Game/Characters/NPC/Blueprints/WBP_Talk.Update Reply` _aswbp_talk self))

(fn `UserConstructionScript`)