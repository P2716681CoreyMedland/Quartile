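; BP_Brick is an interactable actor that opens ThirdPersonMap when its Interact event fires.
; It creates a P_Interact prompt widget on BeginPlay.
; Box overlap events add the prompt to the viewport when the first player character enters and remove it when that character leaves.
; Interact itself does not check whether the player is inside the box.
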(event `/Game/Carson/Blueprints/BP_Interact.Interact`
  (params (Player :type "Character Object Reference"))
  (`GameplayStatics.OpenLevel` "ThirdPersonMap"))

(event `self.Box.OnComponentBeginOverlap`
  (params (OverlappedComponent :type "PrimitiveComponent Object Reference") (OtherActor :type "Actor Object Reference") (OtherComp :type "PrimitiveComponent Object Reference") (OtherBodyIndex :type Integer) (bFromSweep :type Boolean) (SweepResult :type "HitResult Structure (by ref)"))
  (if (== OtherActor (`GameplayStatics.GetPlayerCharacter` 0))
    (`UserWidget.AddToViewport` (`self.InteractWidget`) 0)))

(event `self.Box.OnComponentEndOverlap`
  (params (OverlappedComponent :type "PrimitiveComponent Object Reference") (OtherActor :type "Actor Object Reference") (OtherComp :type "PrimitiveComponent Object Reference") (OtherBodyIndex :type Integer))
  (if (== (`GameplayStatics.GetPlayerCharacter` 0) OtherActor)
    (`Widget.RemoveFromParent` (`self.InteractWidget`))))

(event `self.ReceiveBeginPlay`
  (bind _returnvalue (`|CreateWidget` "/Game/Carson/Blueprints/P_Interact.P_Interact_C"))
  (set `self.InteractWidget` _returnvalue))

(fn `UserConstructionScript`)