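; BlueButton is a trigger button that activates only after the red and green buttons are already set.
; It shows BlueMat on its Cube at BeginPlay.
; Any overlap with its Sphere checks the RedButton and GreenButton flags on GM_QuadGame, then sets BlueButton there and switches the Cube to PaintMat.
; The game mode holds the shared button state, and this Blueprint never clears it.
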(event `self.ReceiveBeginPlay`
  (`PrimitiveComponent.SetMaterial` (`self.Cube`) 0 "/Game/Player/Materials/BlueMat.BlueMat"))

(event `self.Sphere.OnComponentBeginOverlap`
  (params (OverlappedComponent :type "PrimitiveComponent Object Reference") (OtherActor :type "Actor Object Reference") (OtherComp :type "PrimitiveComponent Object Reference") (OtherBodyIndex :type Integer) (bFromSweep :type Boolean) (SweepResult :type "HitResult Structure (by ref)"))
  (bind _asgm_quad_game (cast `/Game/Player/GM_QuadGame` (`GameplayStatics.GetGameMode`) :!pure true))
  (if (and (`/Game/Player/GM_QuadGame.RedButton` _asgm_quad_game) (`/Game/Player/GM_QuadGame.GreenButton` _asgm_quad_game))
    (set `/Game/Player/GM_QuadGame.BlueButton` true _asgm_quad_game)
    (`PrimitiveComponent.SetMaterial` (`self.Cube`) 0 "/Game/Player/Materials/PaintMat.PaintMat")))

(fn `UserConstructionScript`)