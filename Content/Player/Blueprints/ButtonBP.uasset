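; ButtonBP is a pressable button that reports its activation to the GM_QuadGame game mode.
; It starts with a red Cube and turns it green when anything begins overlapping its Sphere.
; The overlap sets the game mode's Button1 flag, or Button2 if Button1 is already set, so flags follow trigger order.
; It has no per-instance guard, so re-entering the same button also sets Button2.
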(event `self.ReceiveBeginPlay`
  (`PrimitiveComponent.SetMaterial` (`self.Cube`) 0 "/Game/Player/Materials/RedMat.RedMat"))

(event `self.Sphere.OnComponentBeginOverlap`
  (params (OverlappedComponent :type "PrimitiveComponent Object Reference") (OtherActor :type "Actor Object Reference") (OtherComp :type "PrimitiveComponent Object Reference") (OtherBodyIndex :type Integer) (bFromSweep :type Boolean) (SweepResult :type "HitResult Structure (by ref)"))
  (bind _asgm_quad_game (cast `/Game/Player/GM_QuadGame` (`GameplayStatics.GetGameMode`) :!pure true))
  (if (`/Game/Player/GM_QuadGame.Button1` _asgm_quad_game)
    (set `/Game/Player/GM_QuadGame.Button2` true _asgm_quad_game)
    (else
      (set `/Game/Player/GM_QuadGame.Button1` true _asgm_quad_game)))
  (`PrimitiveComponent.SetMaterial` (`self.Cube`) 0 "/Game/Player/Materials/GreenMat.GreenMat"))

(fn `UserConstructionScript`)