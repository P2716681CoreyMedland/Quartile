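; DoorBP is a door actor that opens by removing itself from the level once two buttons are active.
; Every tick it casts the game mode to GM_QuadGame and polls its Button1 and Button2 flags.
; When both are true and DoorOpen is unset, OpenDoor sets the flag and destroys the actor, with no animation or way to close again.
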(event `self.ReceiveTick`
  (params (DeltaSeconds :type "Float (single-precision)"))
  (bind _asgm_quad_game (cast `/Game/Player/GM_QuadGame` (`GameplayStatics.GetGameMode`) :!pure true))
  (if (and (and (`/Game/Player/GM_QuadGame.Button1` _asgm_quad_game) (`/Game/Player/GM_QuadGame.Button2` _asgm_quad_game)) (not (`self.DoorOpen`)))
    (`self.OpenDoor`)))

(event `OpenDoor`
  (set `self.DoorOpen` true)
  (`self.K2_DestroyActor`))

(fn `UserConstructionScript`)