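; Game mode for the Quad game that manages the HUD, the pause menu and a running timer.
; On BeginPlay it creates the HUD widget for the first player controller and adds it to the viewport.
; A ShowPauseMenu event does the same for the pause menu, reusing the stored widget when valid.
; Tick accumulates delta seconds into the Timer variable.
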(event `self.ReceiveBeginPlay`
  ;[1 1 1] Show Main Menu
  (`/Engine/EditorBlueprintResources/StandardMacros.IsValid` (`self.HUD_WB`)
    (:`Is Valid`
      _)
    (:`Is Not Valid`
      (bind _returnvalue (`|CreateWidget` "/Game/Player/Widgets/HUD.HUD_C" (`GameplayStatics.GetPlayerController` 0)))
      (set `self.HUD_WB` _returnvalue)))
  (`UserWidget.AddToViewport` (`self.HUD_WB`) 0))

(event `self.ReceiveTick`
  (params (DeltaSeconds :type "Float (single-precision)"))
  ;[1 1 1] Increment Timer
  (set `self.Timer` (+ DeltaSeconds (`self.Timer`))))

(event `ShowPauseMenu`
  ;[1 1 1] Show Pause Menu
  (`/Engine/EditorBlueprintResources/StandardMacros.IsValid` (`self.PauseMenuWB`)
    (:`Is Valid`
      _)
    (:`Is Not Valid`
      (bind _returnvalue (`|CreateWidget` "/Game/Player/Widgets/PauseMenu.PauseMenu_C" (`GameplayStatics.GetPlayerController` 0)))
      (set `self.PauseMenuWB` _returnvalue)))
  (`UserWidget.AddToViewport` (`self.PauseMenuWB`) 0))

(fn `UserConstructionScript`)